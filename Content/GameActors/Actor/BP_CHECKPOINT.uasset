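; BP_CHECKPOINT is a checkpoint actor that registers itself as the player character Till's respawn point.
; When flagged as the default respawn, it registers itself with Till on BeginPlay.
; When Till's capsule overlaps the trigger box, it becomes the new checkpoint, activates its set of fire VFX and turns on its point light.
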(event `self.ReceiveBeginPlay`
  (if (`self.DefaultRespawn`)
    (`/Game/BPs_Characters/Blueprints/BP_PlayerCharacter.New Checkpoint` (`/Game/GameActors/Actor/BP_QOL.Get Till`) self)))

(event `self.TriggerCheckpointBox.OnComponentBeginOverlap`
  (params (OverlappedComponent :type "PrimitiveComponent Object Reference") (OtherActor :type "Actor Object Reference") (OtherComp :type "PrimitiveComponent Object Reference") (OtherBodyIndex :type Integer) (bFromSweep :type Boolean) (SweepResult :type "HitResult Structure (by ref)"))
  (bind _asbp_player_character (`/Game/GameActors/Actor/BP_QOL.Get Till`))
  (if (== (`Character.CapsuleComponent` _asbp_player_character) OtherComp)
    (`/Game/BPs_Characters/Blueprints/BP_PlayerCharacter.New Checkpoint` _asbp_player_character self)
    (`ActorComponent.Activate` (`self.VFX_Fire_CHECKPOINT3`) false)
    (`ActorComponent.Activate` (`self.VFX_Fire_CHECKPOINT7`) false)
    (`ActorComponent.Activate` (`self.VFX_Fire_CHECKPOINT`) false)
    (`ActorComponent.Activate` (`self.VFX_Fire_CHECKPOINT1`) false)
    (`ActorComponent.Activate` (`self.VFX_Fire_CHECKPOINT2`) false)
    (`ActorComponent.Activate` (`self.VFX_Fire_CHECKPOINT6`) false)
    (`ActorComponent.Activate` (`self.VFX_Fire_CHECKPOINT5`) false)
    (`ActorComponent.Activate` (`self.VFX_Fire_CHECKPOINT4`) false)
    (`SceneComponent.SetVisibility` (`self.PointLight`) true false)))

(fn `UserConstructionScript`)