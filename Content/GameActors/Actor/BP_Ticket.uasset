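; BP_Ticket is a collectible ticket actor that the character Till picks up by touch.
; When the Cube component overlaps Till's capsule, the ticket hides itself, plays a 2D pickup sound and disables its collision.
; It then adds its CollectibleAmount to the CollectibleCount stored in BP_GameInstance.
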(event `self.Cube.OnComponentBeginOverlap`
  (params (OverlappedComponent :type "PrimitiveComponent Object Reference") (OtherActor :type "Actor Object Reference") (OtherComp :type "PrimitiveComponent Object Reference") (OtherBodyIndex :type Integer) (bFromSweep :type Boolean) (SweepResult :type "HitResult Structure (by ref)"))
  ;[1 1 1] Collectible System
  (if (== OtherComp (`Character.CapsuleComponent` (`/Game/GameActors/Actor/BP_QOL.Get Till`)))
    (`self.SetActorHiddenInGame` true)
    (`GameplayStatics.PlaySound2D` "/Game/Sound/Clefs/clefs_7.clefs_7" 1.0 1.0 0.0 null null)
    (`self.SetActorEnableCollision` false)
    (bind _asbp_game_instance (cast `/Game/BPs_Characters/Blueprints/GameInstance/BP_GameInstance` (`GameplayStatics.GetGameInstance`)))
    (set `/Game/BPs_Characters/Blueprints/GameInstance/BP_GameInstance.CollectibleCount` (+ (`/Game/BPs_Characters/Blueprints/GameInstance/BP_GameInstance.CollectibleCount` _asbp_game_instance) (`self.CollectibleAmount`)) _asbp_game_instance)))

(fn `UserConstructionScript`)